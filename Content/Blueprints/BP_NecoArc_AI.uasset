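; Boss enemy character for Neco Arc, with health, melee and ranged attacks, and an explosive death.
; Damage updates the player's boss health bar, then either grants brief invincibility or sets the IsDead blackboard key and plays death.
; Melee montages use per-attack values for HitDetect's forward dash, socket sphere trace, damage and knockback.
; The throw montage starts a cooldown, and CreateProjectile spawns a player-targeted projectile from the right hand.
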(event Custom|Attack
  ;[1 1 1] Attack
  (CallFunction|SetAttackValues)
  (Animation|Montage|PlayMontage (Variables|Character|GetMesh) (Utilities|Select :Index (Variables|Attacking|GetAttackSelection) :NewEnumerator0 "/Game/Characters/necoarc/animations/Right_Swipe_Montage.Right_Swipe_Montage" :NewEnumerator1 "/Game/Characters/necoarc/animations/Drop_Kick_Montage.Drop_Kick_Montage" :NewEnumerator2 "/Game/Characters/necoarc/animations/Double_Swipe_Montage.Double_Swipe_Montage") 1.5
    (:OnCompleted
      _)
    (:OnInterrupted
      _))
  (Default|CallOnAttackEnd))

(event Custom|Invincibility
  ;[1 1 1] Invincibility
  (Variables|Actor|SetbCanBeDamaged false)
  (Utilities|FlowControl|Delay (Variables|Default|GetIFrames))
  (Variables|Actor|SetbCanBeDamaged true))

(event Custom|Die
  (bind _returnvalue (Transformation|GetActorLocation))
  ;[1 1 1] Die
  (Utilities|FlowControl|DoOnce false
    (:Completed
      (AI|ClearFocus (AI|GetAIController self))
      (Animation|Montage|PlayMontage (Variables|Character|GetMesh) "/Game/Characters/necoarc/animations/Mutant_Dying_Montage.Mutant_Dying_Montage" 1.0 0.5
        (:OnNotifyBegin
          (Actor|DestroyActor)
          (Audio|PlaySoundatLocation "/Game/StarterContent/Audio/Explosion01.Explosion01" _returnvalue "0, 0, 0" 1.0 1.0 0.0 0 0 0 0)
          (Effects|SpawnEmitteratLocation "/Game/StarterContent/Particles/P_Explosion.P_Explosion" _returnvalue "0, 0, 0" "5.000000,5.000000,5.000000"))))))

(event Custom|CreateProjectile
  ;[1 1 1] Ranged Attack
  (bind _returnvalue (Actor|GetActorOfClass "/Game/ThirdPerson/Blueprints/BP_ThirdPersonCharacter.BP_ThirdPersonCharacter_C"))
  (Game|SpawnActorfromClass "/Game/Projectiles/BP_Projectile.BP_Projectile_C" (Transformation|GetSocketTransform (Variables|Character|GetMesh) "RightHand" "RTS_World") "Undefined" "MultiplyWithRoot" self 2e+03 0.0 _returnvalue 1e+01 0))

(event Custom|RangedAttack
  ;[1 1 1] Ranged Attack
  (Animation|Montage|PlayMontage (Variables|Character|GetMesh) "/Game/Characters/necoarc/animations/Throw_Object_Montage.Throw_Object_Montage"
    (:OnCompleted
      _)
    (:OnInterrupted
      _))
  (Default|CallOnAttackEnd)
  (Variables|RangedAttack|SetRangedAttackAvailable false)
  (Utilities|FlowControl|Delay (Variables|RangedAttack|GetRangedAttackCooldown))
  (Variables|RangedAttack|SetRangedAttackAvailable true))

(event EventBeginPlay
  (AddComponent|AddBlackboardComponent))

(event Game|Damage|EventAnyDamage
  (params (Damage :type Float%20%28single-precision%29) (DamageType :type Damage%20Type%20Object%20Reference) (InstigatedBy :type Controller%20Object%20Reference) (DamageCauser :type Actor%20Object%20Reference))
  ;[1 1 1] Health
  (Variables|Stats|SetCurrentHealth (Math|Float|Clamp(Float) (- (Variables|Stats|GetCurrentHealth) Damage) 0.0 (Variables|Stats|GetMaxHealth)))
  (bind _asbp_third_person_character (Utilities|Casting|CastToBP_ThirdPersonCharacter (Game|GetPlayerCharacter 0)))
  (Default|UpdateBossHealthBar _asbp_third_person_character (Variables|Stats|GetCurrentHealth) (Variables|Stats|GetMaxHealth))
  (if (== (Variables|Stats|GetCurrentHealth) 0.0)
    (AI|Components|Blackboard|SetValueasBool (AI|GetBlackboard 0) (Utilities|Name|MakeLiteralName "IsDead") true)
    (CallFunction|Die)
    (else
      (CallFunction|Invincibility))))

(fn ConstructionScript
  (Variables|Stats|SetCurrentHealth (Variables|Stats|GetMaxHealth)))

(fn HitDetect
  (bind _attackselection (Variables|Attacking|GetAttackSelection))
  (bind _double_swipe_bone (Variables|Attacking|GetDouble%20Swipe%20Bone))
  (bind _mesh (Variables|Character|GetMesh))
  (bind _returnvalue (Utilities|Select :Index _attackselection :NewEnumerator0 "RightHand" :NewEnumerator1 "Hips" :NewEnumerator2 _double_swipe_bone))
  (bind _returnvalue_2 (Transformation|GetSocketLocation _mesh _returnvalue))
  (Character|LaunchCharacter (* (Transformation|GetActorForwardVector) (Variables|Attacking|GetAttackDashDistance)) false false) ; Character Dashes Forward
  (bind _outhit (Collision|SphereTraceForObjects _returnvalue_2 _returnvalue_2 (Variables|Stats|GetHurtboxSize) (Utilities|Array|MakeArray "ObjectTypeQuery3") false 0 "Persistent"))
  (bind _returnvalue_3 (Game|Damage|ApplyDamage (.HitActor (Collision|BreakHitResult _outhit)) (* (Variables|Stats|GetBaseDamage) (Variables|Stats|GetDamageMultiplier)) 0 self))
  (if (>= _returnvalue_3 0.0)
    (bind _ascharacter (Utilities|Casting|CastToCharacter (.HitActor (Collision|BreakHitResult _outhit))))
    (Character|LaunchCharacter _ascharacter (* (Transformation|GetActorForwardVector) (Variables|Attacking|GetAttackLaunchDistance)) false false)))

(fn SetAttackValues
  (switch Utilities|FlowControl|Switch|SwitchonENecoArc_Attacks (Variables|Attacking|GetAttackSelection)
    (:NewEnumerator0
      (Variables|Attacking|SetAttackDashDistance 9e+01 :!label _label)
      (Variables|Attacking|SetAttackLaunchDistance 1e+02)
      (Variables|Stats|SetDamageMultiplier 1.0)
      (Variables|Stats|SetHurtboxSize 1.2e+02))
    (:NewEnumerator1
      (Variables|Attacking|SetAttackDashDistance 3e+02)
      (Variables|Attacking|SetAttackLaunchDistance 1.5e+02)
      (Variables|Stats|SetDamageMultiplier 2.0)
      (Variables|Stats|SetHurtboxSize 2e+02))
    (:NewEnumerator2
      (goto _label))))